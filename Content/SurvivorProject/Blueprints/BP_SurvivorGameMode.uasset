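; Game mode for a survivor game that runs endless enemy spawning, tracks kills and handles player death.
; On BeginPlay it creates the HUD and binds the player's death to enabling the HUD's reset button.
; A delay loop spawns enemies at a random angle and set distance around the player, shortening the interval toward a minimum.
; Each enemy's death event increments the kill count shown on the HUD.
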(event Custom|OnEnemyDead
  (bind _result (Math|Integer|IncrementInt (Variables|Default|GetCount))
    (:%20%20
      (Default|UpdateKillCount (Variables|Default|GetHUDWidget) _result))))

(event Custom|OnPlayerDead
  (Default|EnableResetButton (Variables|Default|GetHUDWidget)))

(event EventBeginPlay
  (Utilities|FlowControl|Sequence
    (:then_0
      (bind _output_get (Variables|Default|SetPlayerPawn (Game|Player|GetPlayerPawn 0)))
      (bind _asplayer_controller (Utilities|Casting|CastToPlayerController (Pawn|GetController _output_get)))
      (bind _returnvalue (UserInterface|CreateWidget "/Game/SurvivorProject/UI/WBP_HUD.WBP_HUD_C" _asplayer_controller))
      (Variables|Default|SetHUDWidget _returnvalue)
      (UserInterface|Viewport|AddtoViewport _returnvalue 0))
    (:then_1
      (bind _assurvivor_character (Utilities|Casting|CastToSurvivorCharacter (Variables|Default|GetPlayerPawn)))
      (Variables|/Script/SurvivorProject.SurvivorCharacter|SetOnDead _assurvivor_character (delegate Custom|OnPlayerDead)))
    (:then_2
      (bind _returnvalue_2 (Game|SpawnActorfromClass (Variables|Default|GetEnemyActor) (Math|Transform|MakeTransform (+ (Transformation|GetActorLocation (Variables|Default|GetPlayerPawn)) (Math|Vector|RotateVector (Math|Vector|MakeVector (Variables|Default|GetDistance) 0.0 0.0) (Math|Rotator|MakeRotator 0.0 0.0 (- (* (Math|Random|RandomFloat) 3.6e+02) 1.8e+02)))) "0, 0, 0" "1.000000,1.000000,1.000000") "AlwaysSpawn" "MultiplyWithRoot" 0 0 :!label _label))
      (bind _assurvivor_enemy_character (Utilities|Casting|CastToSurvivorEnemyCharacter _returnvalue_2))
      (Variables|/Script/SurvivorProject.SurvivorEnemyCharacter|SetOnDead _assurvivor_enemy_character (delegate Custom|OnEnemyDead))
      (Utilities|FlowControl|Delay (Variables|Default|GetSpawnDelay))
      (Variables|Default|SetSpawnDelay (Math|Float|Max(Float) (- (Variables|Default|GetSpawnDelay) (Variables|Default|GetSpawnDelayShrink)) (Variables|Default|GetMinSpawnDelay)))
      (goto _label))))

(event EventTick
  (params (DeltaSeconds :type Float%20%28single-precision%29)))

(fn ConstructionScript)